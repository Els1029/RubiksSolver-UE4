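; BP_cubeDetector reads a video feed to capture cube faces and colours, apparently for a Rubik's-style puzzle.
; Each frame feeds a dynamic material on the Cube component, while the Capture input sets a colour or captures a face, depending on Recalibrate or Detect mode.
; Update events refresh the colour, face and cube displays, and test inputs rotate the current face or cube.
; The RecalibrateColours widget creation is unwired.
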(event `self.ReceiveBeginPlay`
  (bind _returnvalue (`PrimitiveComponent.CreateDynamicMaterialInstance` (`self.Cube`) 0 "/Game/CamMat.CamMat" "None"))
  (bind _output_get (set `self.DynMat` _returnvalue))
  (`PrimitiveComponent.SetMaterial` (`self.Cube`) 0 _output_get)
  (`self.BeginCapture`))

(event `self.OnNextVideoFrame`
  (`MaterialInstanceDynamic.SetTextureParameterValue` (`self.DynMat`) "CamTexture" (`self.VideoTexture`)))

(event `InputAction|Capture`
  (params (Key :type "Key Structure"))
  (:`Released`
    (if (select `captureMode` (`self.currentMode`) :`Recalibrate` true)
      (`self.setColor`)
      (else
        (`self.captureFace`)))))

(event `self.colourUpdated`
  (`/Game/CubeDisplay/RecalibrateColours.Update Colours` (`self.RecalibrateColours`)))

(event `self.modeUpdated`
  (if (not (select `captureMode` (`self.currentMode`) :`Recalibrate` true))
    (`/Game/CubeDisplay/colourUpdater.Colours Done` (`self.colourUpdater`))))

(event `self.targetColourUpdated`
  (bind _colourtargets (`self.colourTargets`))
  (bind _facedisplay (`self.FaceDisplay`))
  (set `/Game/CubeDisplay/currentDetectedFace.Colours` _colourtargets _facedisplay)
  (`/Game/CubeDisplay/currentDetectedFace.colourUpdated` _facedisplay)
  (`/Game/CubeDisplay/currentColours.Update Colours` (`self.currentColours`) _colourtargets))

(event `self.faceDetected`
  (`/Game/CubeDisplay/currentDetectedFace.face Updated` (`self.FaceDisplay`) (`self.currentFace`) :!label _label))

(event `InputAction|rotateTest`
  (params (Key :type "Key Structure"))
  (:`Released`
    (bind _returnvalue (`CubeFunctions.rotateFaceCW` (`self.currentFace`)))
    (set `self.currentFace` _returnvalue)
    (goto _label)))

(event `self.cubeUpdated`
  (`/Game/CubeDisplay/cubeWidget.cubeUpdated` (`self.CubeDisplay`) (`self.currentCube`) :!label _label_2))

(event `InputAction|rotateCubeTest`
  (params (Key :type "Key Structure"))
  (:`Pressed`
    (`CubeFunctions.rotateCube` (`self.currentCube`) "F")
    (goto _label_2)))

(fn `UserConstructionScript`)